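; BP_Portal_Entry is the portal that sends players into the duel arena.
; On sphere overlap it looks for an available random "into-arena" locator, retrying after a delay, and teleports the actor to the stored spawn location.
; It applies arena and infinite-bubble gameplay effects to the player, announces the join on authority and plays teleport effects.
; It updates the GameState's arena count, announcing and starting the duel timer once two players fill it.
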(event `GrabArenaSpawnLocation`
  (bind _outactors (`GameplayStatics.GetAllActorsOfClassWithTag` "/Game/_MageryWars/Blueprints/BP_Portal_Entry_Locator.BP_Portal_Entry_Locator_C" "into-arena"))
  (bind _output (`|GetArrayItem` _outactors (`KismetMathLibrary.RandomInteger` (`KismetArrayLibrary.Array_Length` _outactors))))
  (if (`/Game/_MageryWars/Blueprints/BP_Portal_Entry_Locator.Available?` _output)
    (set `self.SpawnLocation` (`self.K2_GetActorLocation` _output))
    (`/Game/_MageryWars/Blueprints/BP_Portal_Entry_Locator.SetNotAvailable` _output)
    (else
      (`KismetSystemLibrary.Delay` 0.2)
      (`self.GrabArenaSpawnLocation`))))

(event `self.ReceiveBeginPlay`
  (bind _asbp_player_controller (cast `/Game/_MageryWars/Blueprints/BP_PlayerController` (`GameplayStatics.GetPlayerController` 0)))
  (set `self.LocalPlayerController` _asbp_player_controller)
  (bind _asbp_game_state (cast `/Game/_MageryWars/Modes/Game/BP_GameState` (`GameplayStatics.GetGameState`)))
  (set `self.GameState` _asbp_game_state))

(event `self.Sphere.OnComponentBeginOverlap`
  (params (OverlappedComponent :type "PrimitiveComponent Object Reference") (OtherActor :type "Actor Object Reference") (OtherComp :type "PrimitiveComponent Object Reference") (OtherBodyIndex :type Integer) (bFromSweep :type Boolean) (SweepResult :type "HitResult Structure (by ref)"))
  (`|ExecutionSequence`
    (:`then_0`
      (`self.GrabArenaSpawnLocation`))
    (:`then_1`
      (`self.K2_SetActorLocation` OtherActor (`self.SpawnLocation`) false true)
      (bind _asbp_player_character (cast `/Game/_MageryWars/Blueprints/BP_PlayerCharacter` OtherActor))
      (bind _returnvalue (`AbilitySystemBlueprintLibrary.GetAbilitySystemComponent` _asbp_player_character))
      (`AbilitySystemComponent.BP_ApplyGameplayEffectToSelf` :`self` _returnvalue :`GameplayEffectClass` "/Game/_MageryWars/Abilities/_Arena/GE_IntoArena.GE_IntoArena_C")
      (`AbilitySystemComponent.BP_ApplyGameplayEffectToSelf` :`self` _returnvalue :`GameplayEffectClass` "/Game/_MageryWars/Abilities/Bubble/GE_BubbleInfinite.GE_BubbleInfinite_C")
      (`/Engine/EditorBlueprintResources/ActorMacros.Switch Has Authority`
        (:`Authority`
          (`/Game/_MageryWars/Blueprints/BP_PlayerController.SERVER_Announcement` (`self.LocalPlayerController`) (`|FormatText` "Arena Master: {player} has joined the arena!" (`/Game/_MageryWars/Blueprints/BP_PlayerCharacter.PlayerName` _asbp_player_character))))))
    (:`then_2`
      (`GameplayStatics.PlaySoundAtLocation` "/Game/_MageryWars/Sounds/teleport.teleport" (`self.K2_GetActorLocation`) (struct) 1.0 1.0 0.0 null null null null)
      (`KismetSystemLibrary.Delay` 0.2)
      (`NiagaraFunctionLibrary.SpawnSystemAtLocation` "/Game/MixedVFX/Particles/Slashes/SeparateParts/Slashes/NS_VampireSlash_OnlySlash.NS_VampireSlash_OnlySlash" (`self.K2_GetActorLocation` OtherActor)))
    (:`then_3`
      (`self.UpdateArena`))))

(event `UpdateArena`
  (`/Game/_MageryWars/Modes/Game/BP_GameState.UpdateAmountOfPlayersInArena` (`self.GameState`) 1)
  (if (`/Game/_MageryWars/Modes/Game/BP_GameState.CheckIfArenaIsFull` (`self.GameState`) 2)
    (`/Game/_MageryWars/Blueprints/BP_PlayerController.SERVER_Announcement` (`self.LocalPlayerController`) "Arena Master: The duel will start in 10 seconds!")
    (`self.StartTimer`)))

(event `StartTimer`
  (`/Game/_MageryWars/Modes/Game/BP_GameState.StartDuelTimer` (`self.GameState`)))

(fn `UserConstructionScript`)