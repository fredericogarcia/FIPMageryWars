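; Arena exit portal that handles a player character leaving the duel arena when it overlaps the sphere.
; If the arena is not full, it moves the player to their respawn location, while the authority announces the departure and decrements the GameState arena count.
; If full with a duel started, it announces a forfeit and applies GE_Chicken through GAS instead.
; Teleport sound and slash Niagara effect follow.
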(event `self.Sphere.OnComponentBeginOverlap`
  (params (OverlappedComponent :type "PrimitiveComponent Object Reference") (OtherActor :type "Actor Object Reference") (OtherComp :type "PrimitiveComponent Object Reference") (OtherBodyIndex :type Integer) (bFromSweep :type Boolean) (SweepResult :type "HitResult Structure (by ref)"))
  (`|ExecutionSequence`
    (:`then_0`
      (bind _asbp_player_character (cast `/Game/_MageryWars/Blueprints/BP_PlayerCharacter` OtherActor))
      (`self.UpdateArena` (`/Game/_MageryWars/Blueprints/BP_PlayerCharacter.PlayerName` _asbp_player_character) _asbp_player_character))
    (:`then_1`
      (if (`self.ShouldPlayerTeleport`)
        (`GameplayStatics.PlaySoundAtLocation` "/Game/_MageryWars/Sounds/Spells/teleport.teleport" (`self.K2_GetActorLocation`) (struct) 1.0 1.0 0.0 null null null null)
        (`KismetSystemLibrary.Delay` 0.2)
        (`NiagaraFunctionLibrary.SpawnSystemAtLocation` "/Game/MixedVFX/Particles/Slashes/SeparateParts/Slashes/NS_VampireSlash_OnlySlash.NS_VampireSlash_OnlySlash" (`self.K2_GetActorLocation` OtherActor))
        (set `self.ShouldPlayerTeleport` false)))))

(event `self.ReceiveBeginPlay`
  (bind _asbp_player_controller (cast `/Game/_MageryWars/Blueprints/BP_PlayerController` (`GameplayStatics.GetPlayerController` 0)))
  (set `self.LocalPlayerController` _asbp_player_controller)
  (bind _asbp_game_state (cast `/Game/_MageryWars/Modes/Game/BP_GameState` (`GameplayStatics.GetGameState`)))
  (set `self.GameState` _asbp_game_state))

(event `UpdateArena`
  (params (PlayerName :type String) (PlayerCharacter :type "/Game/_MageryWars/Blueprints/BP_PlayerCharacter Object Reference"))
  (if (`/Game/_MageryWars/Modes/Game/BP_GameState.CheckIfArenaIsFull` (`self.GameState`) 2)
    (set `self.ShouldPlayerTeleport` true)
    (if (`/Game/_MageryWars/Modes/Game/BP_GameState.DuelStarted` (`self.GameState`))
      (`/Game/_MageryWars/Blueprints/BP_PlayerController.SERVER_Announcement` (`self.LocalPlayerController`) (`|FormatText` "{player} has forfeited the match!" PlayerName))
      (`AbilitySystemComponent.BP_ApplyGameplayEffectToSelf` :`self` (`AbilitySystemBlueprintLibrary.GetAbilitySystemComponent` PlayerCharacter) :`GameplayEffectClass` "/Game/_MageryWars/Abilities/_Arena/GE_Chicken.GE_Chicken_C"))
    (else
      (set `self.ShouldPlayerTeleport` true)
      (`self.K2_SetActorLocation` PlayerCharacter (`/Game/_MageryWars/Blueprints/BP_PlayerCharacter.RespawnLocation` PlayerCharacter) false true)
      (`/Engine/EditorBlueprintResources/ActorMacros.Switch Has Authority`
        (:`Authority`
          (`/Game/_MageryWars/Blueprints/BP_PlayerController.SERVER_Announcement` (`self.LocalPlayerController`) (`|FormatText` "{player} has left the arena!" PlayerName))
          (`/Game/_MageryWars/Modes/Game/BP_GameState.UpdateAmountOfPlayersInArena` (`self.GameState`) -1))))))

(fn `UserConstructionScript`)