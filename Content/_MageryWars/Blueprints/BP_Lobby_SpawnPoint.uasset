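; Lobby spawn point that displays a third-person character for a player assigned to it.
; AddPlayer stores the controller, spawns the character at SpawnLocation raised by its capsule half-height, and sets its name from the lobby game mode.
; If a character already exists, AddPlayer only destroys it without spawning a replacement.
; RemovePlayer clears the controller and destroys the character.
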(event `Add Player`
  (params (PlayerController :type "PlayerController Object Reference"))
  (bind _returnvalue (`SceneComponent.K2_GetComponentToWorld` (`self.SpawnLocation`)))
  (bind _output_get (set `self.PlayerController` PlayerController))
  (bind _lobbycharacter (`self.LobbyCharacter`)
    (:`then`
      (`self.K2_DestroyActor` _lobbycharacter))
    (:`else`
      (bind _returnvalue_2 (`|SpawnActorFromClass` "/Game/ThirdPerson/Blueprints/BP_ThirdPersonCharacter.BP_ThirdPersonCharacter_C" (`SceneComponent.K2_GetComponentToWorld` (`self.SpawnLocation`)) "AlwaysSpawn" "MultiplyWithRoot" _output_get null))
      (bind _output_get_2 (set `self.LobbyCharacter` _returnvalue_2))
      (`self.K2_SetActorTransform` _output_get_2 (`KismetMathLibrary.MakeTransform` (`KismetMathLibrary.MakeVector` (.x (.location _returnvalue)) (.y (.location _returnvalue)) (+ (`CapsuleComponent.GetScaledCapsuleHalfHeight` (`Character.CapsuleComponent` _returnvalue_2)) (.z (.location _returnvalue)))) (.rotation _returnvalue) (.scale _returnvalue)) false false)
      (`self.SetOwner` (`self.LobbyCharacter`))
      (bind _asbp_lobby_game_mode (cast `/Game/_MageryWars/Modes/Lobby/BP_Lobby_GameMode` (`GameplayStatics.GetGameMode`)))
      (set `/Game/ThirdPerson/Blueprints/BP_ThirdPersonCharacter.Player Name` (`KismetTextLibrary.Conv_StringToText` (`/Game/_MageryWars/Modes/Lobby/BP_Lobby_GameMode.GetPlayerName` _asbp_lobby_game_mode (`self.PlayerController`))) (`self.LobbyCharacter`)))))

(event `Remove Player`
  (set `self.PlayerController` null)
  (bind _lobbycharacter (`self.LobbyCharacter`)
    (:`then`
      (`self.K2_DestroyActor` _lobbycharacter)
      (set `self.LobbyCharacter` null))
    (:`else`)))

(fn `UserConstructionScript`)