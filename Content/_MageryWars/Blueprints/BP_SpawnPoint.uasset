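; BP_SpawnPoint is a spawn point that holds one player controller and the third-person character representing that player.
; AddPlayer spawns the character at SpawnLocation, raises it by its capsule half-height and sets its name from the player's Steam persona.
; If a character already exists, AddPlayer only destroys it without spawning a replacement.
; RemovePlayer clears the controller and destroys any existing character.
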(event `Add Player`
  (params (PlayerController :type "PlayerController Object Reference"))
  (bind _returnvalue (`SceneComponent.K2_GetComponentToWorld` (`self.SpawnLocation`)))
  (set `self.PlayerController` PlayerController)
  (bind _character (`self.Character`)
    (:`then`
      (`self.K2_DestroyActor` _character))
    (:`else`
      (bind _returnvalue_2 (`|SpawnActorFromClass` "/Game/ThirdPerson/Blueprints/BP_ThirdPersonCharacter.BP_ThirdPersonCharacter_C" (`SceneComponent.K2_GetComponentToWorld` (`self.SpawnLocation`)) "AlwaysSpawn" "MultiplyWithRoot" null null))
      (bind _output_get (set `self.Character` _returnvalue_2))
      (`self.K2_SetActorTransform` _output_get (`KismetMathLibrary.MakeTransform` (`KismetMathLibrary.MakeVector` (.x (.location _returnvalue)) (.y (.location _returnvalue)) (+ (`CapsuleComponent.GetScaledCapsuleHalfHeight` (`Character.CapsuleComponent` _returnvalue_2)) (.z (.location _returnvalue)))) (.rotation _returnvalue) (.scale _returnvalue)) false false)
      (bind _returnvalue_3 (`AdvancedSteamFriendsLibrary.GetSteamPersonaName` (`AdvancedSessionsLibrary.GetUniqueNetID` (`self.PlayerController`))))
      (set `/Game/ThirdPerson/Blueprints/BP_ThirdPersonCharacter.Player Name` (`KismetTextLibrary.Conv_StringToText` _returnvalue_3) (`self.Character`)))))

(event `Remove Player`
  (set `self.PlayerController` null)
  (bind _character (`self.Character`)
    (:`then`
      (`self.K2_DestroyActor` _character)
      (set `self.Character` null))
    (:`else`)))

(fn `UserConstructionScript`)