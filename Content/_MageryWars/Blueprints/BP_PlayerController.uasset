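; Player controller for Magery Wars that creates the local player's HUD and handles multiplayer text chat.
; After HUD creation, it announces the player joining, using the GameInstance name or a random numbered fallback.
; Messages and announcements go through server events, which loop over the GameState PlayerArray and call a client event on each controller to fill the HUD chat.
; The chat input action focuses the chat text box.
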(event `self.ReceiveBeginPlay`
  (`KismetSystemLibrary.DelayUntilNextTick`)
  ;[1 0.4912 0] Is Locally Controlled
  (if (`self.IsLocalPlayerController`)
    ; Comment
    (bind _returnvalue (`|CreateWidget` "/Game/_MageryWars/Widgets/W_HUD.W_HUD_C" self))
    (set `self.W_HUD` _returnvalue)
    (`UserWidget.AddToViewport` _returnvalue 0)
    (`KismetSystemLibrary.DelayUntilNextTick`)
    (`self.GetPlayerNameAndAnnounceIt`)))

(event `CLIENT_CreateMessage`
  (params (Message :type Text))
  ;[0.01764 0 0.0087] Multiplayer Chat
  (bind _w_hud (`self.W_HUD`)
    (:`then`
      (`/Game/_MageryWars/Widgets/W_Chat.CreateMessageWidget` (`/Game/_MageryWars/Widgets/W_HUD.W_Chat` _w_hud) Message))
    (:`else`)))

(event `SERVER_SubmitMessage`
  (params (Message :type Text))
  ;[0.01764 0 0.0087] Multiplayer Chat
  (for _array_element (`GameStateBase.PlayerArray` (`GameplayStatics.GetGameState`))
    (bind _asbp_player_controller (cast `/Game/_MageryWars/Blueprints/BP_PlayerController` (`PlayerState.GetPlayerController` _array_element)))
    (`self.CLIENT_CreateMessage` _asbp_player_controller Message)))

(event `SERVER_Announcement`
  (params (Message :type Text))
  ;[0.01764 0 0.0087] Multiplayer Chat
  (`self.SERVER_SubmitMessage` Message))

(event `EnhancedInput|/Game/ThirdPerson/Input/Actions/IA_Chat`
  (params (ActionValue :type Boolean) (ElapsedSeconds :type "Float (double-precision)") (TriggeredSeconds :type "Float (double-precision)") (InputAction :type "InputAction Object Reference" :default "/Game/ThirdPerson/Input/Actions/IA_Chat.IA_Chat"))
  (bind _e_textbox (`/Game/_MageryWars/Widgets/W_Chat.E_TextBox` (`/Game/_MageryWars/Widgets/W_HUD.W_Chat` (`self.W_HUD`))))
  ;[0.01764 0 0.0087] Multiplayer Chat
  (:`Started`
    (`self.W_HUD`
      (:`then`
        (if (not (`Widget.HasKeyboardFocus` _e_textbox))
          (`Widget.SetKeyboardFocus` _e_textbox)))
      (:`else`))))

(fn `GetPlayerNameAndAnnounceIt`
  (`/Engine/EditorBlueprintResources/StandardMacros.DoOnce` false
    (:`Completed`
      (bind _asbp_game_instance (cast `/Game/_MageryWars/Blueprints/BP_GameInstance` (`GameplayStatics.GetGameInstance`))
        (:`then`
          (bind _playername (`/Game/_MageryWars/Blueprints/BP_GameInstance.PlayerName` _asbp_game_instance))
          (if (`KismetStringLibrary.IsEmpty` _playername)
            (set `self.Player Name` (`KismetTextLibrary.Conv_TextToString` (`|FormatText` "Player {x}" (`KismetMathLibrary.RandomInteger` 99))))
            (else
              (set `self.Player Name` _playername)))
          ;[0.3366 0 1] Server announcement
          (`self.SERVER_Announcement` (`|FormatText` "{player} has joined the map!" (`self.Player Name`))))
        (:`CastFailed`
          (`KismetSystemLibrary.K2_SetTimer` null "GetPlayerNameAndAnnounceIt" 0.01))))))

(fn `UserConstructionScript`)