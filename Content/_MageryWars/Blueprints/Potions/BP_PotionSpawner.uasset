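; BP_PotionSpawner periodically spawns BP_Potion actors of a configured PotionType at random spots within a box area.
; The construction script sizes SpawnBox from SpawnArea, and SpawnPotion picks random X and Y inside its bounds at a fixed world height.
; A looping 30-second timer starts on BeginPlay, with StartPotionTimer and StopPotionTimer events to restart or clear it.
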(event `SpawnPotion`
  (bind (_origin _boxextent) (`KismetSystemLibrary.GetComponentBounds` (`self.SpawnBox`)))
  (bind (_returnvalue_x _returnvalue_y) (`KismetMathLibrary.BreakVector` (`KismetMathLibrary.RandomPointInBoundingBox` _origin _boxextent)))
  (`|SpawnActorFromClass` "/Game/_MageryWars/Blueprints/Potions/BP_Potion.BP_Potion_C" (`KismetMathLibrary.MakeTransform` (`KismetMathLibrary.MakeVector` _returnvalue_x _returnvalue_y 100.0)) "Undefined" "MultiplyWithRoot" null (`self.Potion Type`) null))

(event `self.ReceiveBeginPlay`
  (bind _returnvalue (`KismetSystemLibrary.K2_SetTimer` null "SpawnPotion" 30.0 true :!label _label))
  (set `self.PotionTimer` _returnvalue))

(event `StartPotionTimer`
  (goto _label))

(event `StopPotionTimer`
  (`KismetSystemLibrary.K2_ClearAndInvalidateTimerHandle` (`self.PotionTimer`)))

(fn `UserConstructionScript`
  (`BoxComponent.SetBoxExtent` (`self.SpawnBox`) (`self.SpawnArea`) true))