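; BP_Potion is a world pickup that restores either health or mana to the player, based on its PotionType.
; On BeginPlay it assigns a matching Niagara effect to its Visual component.
; When a BP_PlayerCharacter overlaps the Box, it applies the corresponding health or mana GameplayEffect through that character's Ability System Component, then destroys itself.
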(event `self.ReceiveBeginPlay`
  (bind _visual (`self.Visual`))
  (switch `/Game/_MageryWars/Blueprints/Potions/E_PotionType` (`self.PotionType`)
    (:`NewEnumerator0`
      (`NiagaraComponent.SetAsset` _visual "/Game/sA_PickupSet_1/Fx/NiagaraSystems/NS_Pickup_3.NS_Pickup_3" true))
    (:`NewEnumerator1`
      (`NiagaraComponent.SetAsset` _visual "/Game/sA_PickupSet_1/Fx/NiagaraSystems/NS_Pickup_2.NS_Pickup_2" true))))

(event `self.Box.OnComponentBeginOverlap`
  (params (OverlappedComponent :type "PrimitiveComponent Object Reference") (OtherActor :type "Actor Object Reference") (OtherComp :type "PrimitiveComponent Object Reference") (OtherBodyIndex :type Integer) (bFromSweep :type Boolean) (SweepResult :type "HitResult Structure (by ref)"))
  (bind _asbp_player_character (cast `/Game/_MageryWars/Blueprints/BP_PlayerCharacter` OtherActor))
  (switch `/Game/_MageryWars/Blueprints/Potions/E_PotionType` (`self.PotionType`)
    (:`NewEnumerator0`
      (`AbilitySystemComponent.BP_ApplyGameplayEffectToSelf` :`self` (`AbilitySystemBlueprintLibrary.GetAbilitySystemComponent` _asbp_player_character) :`GameplayEffectClass` "/Game/_MageryWars/Abilities/Potions/GE_HealthPotion.GE_HealthPotion_C"))
    (:`NewEnumerator1`
      (`AbilitySystemComponent.BP_ApplyGameplayEffectToSelf` :`self` (`AbilitySystemBlueprintLibrary.GetAbilitySystemComponent` _asbp_player_character) :`GameplayEffectClass` "/Game/_MageryWars/Abilities/Potions/GE_ManaPotion.GE_ManaPotion_C")))
  (`self.K2_DestroyActor`))

(fn `UserConstructionScript`)