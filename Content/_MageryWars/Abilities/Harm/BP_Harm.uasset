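; BP_Harm is a homing projectile for the Harm ability that applies the GE_Harm gameplay effect to the player character it hits.
; The construction script adds a gravity-free ProjectileMovementComponent that homes on HomingTargetComponent and rotates with its velocity.
; Sphere overlap ignores the owner, has the hit BP_PlayerCharacter's ability system create and self-apply the effect, then destroys the projectile.
; Tick only checks target validity, with no resulting action.
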(event `self.ReceiveTick`
  (params (DeltaSeconds :type "Float (single-precision)"))
  (`self.Homing Target Component`
    (:`then`)
    (:`else`)))

(event `self.Sphere.OnComponentBeginOverlap`
  (params (OverlappedComponent :type "PrimitiveComponent Object Reference") (OtherActor :type "Actor Object Reference") (OtherComp :type "PrimitiveComponent Object Reference") (OtherBodyIndex :type Integer) (bFromSweep :type Boolean) (SweepResult :type "HitResult Structure (by ref)"))
  (if (!= OtherActor (`self.GetOwner`))
    (bind _asbp_player_character (cast `/Game/_MageryWars/Blueprints/BP_PlayerCharacter` OtherActor))
    (bind _returnvalue (`AbilitySystemBlueprintLibrary.GetAbilitySystemComponent` _asbp_player_character))
    (`AbilitySystemComponent.BP_ApplyGameplayEffectSpecToSelf` _returnvalue (`AbilitySystemComponent.MakeOutgoingSpec` :`self` _returnvalue :`GameplayEffectClass` "/Game/_MageryWars/Abilities/Harm/GE_Harm.GE_Harm_C"))
    (`self.K2_DestroyActor`)))

(fn `UserConstructionScript`
  (bind _returnvalue (`AddComponent|NODE_AddProjectileMovementComponent-0`))
  (set `ProjectileMovementComponent.ProjectileGravityScale` 0.0 _returnvalue)
  (set `ProjectileMovementComponent.InitialSpeed` 750.0 _returnvalue)
  (set `ProjectileMovementComponent.MaxSpeed` 1000.0 _returnvalue)
  (set `ProjectileMovementComponent.bIsHomingProjectile` true _returnvalue)
  (set `ProjectileMovementComponent.HomingTargetComponent` (`self.Homing Target Component`) _returnvalue)
  (set `ProjectileMovementComponent.bRotationFollowsVelocity` true _returnvalue)
  (set `ProjectileMovementComponent.HomingAccelerationMagnitude` 10000.0 _returnvalue))