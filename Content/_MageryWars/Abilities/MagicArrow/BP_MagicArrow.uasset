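; BP_MagicArrow is the Magic Arrow ability's projectile, which applies a gameplay effect to the player character it hits.
; The construction script passes HomingTargetComponent to ProjectileMovement as its homing target.
; Sphere overlaps ignore the owner; any other actor destroys the arrow.
; For a BP_PlayerCharacter, the victim's own ability system component makes and self-applies the GameplayEffectClass spec, so the shooter is not the effect's source.
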(event `self.Sphere.OnComponentBeginOverlap`
  (params (OverlappedComponent :type "PrimitiveComponent Object Reference") (OtherActor :type "Actor Object Reference") (OtherComp :type "PrimitiveComponent Object Reference") (OtherBodyIndex :type Integer) (bFromSweep :type Boolean) (SweepResult :type "HitResult Structure (by ref)"))
  (if (!= OtherActor (`self.GetOwner`))
    (bind _asbp_player_character (cast `/Game/_MageryWars/Blueprints/BP_PlayerCharacter` OtherActor)
      (:`then`
        (bind _returnvalue (`AbilitySystemBlueprintLibrary.GetAbilitySystemComponent` _asbp_player_character))
        (`AbilitySystemComponent.BP_ApplyGameplayEffectSpecToSelf` _returnvalue (`AbilitySystemComponent.MakeOutgoingSpec` :`self` _returnvalue :`GameplayEffectClass` (`self.Gameplay Effect Class`)))
        (`self.K2_DestroyActor`))
      (:`CastFailed`
        (`self.K2_DestroyActor`)))))

(fn `UserConstructionScript`
  (set `ProjectileMovementComponent.HomingTargetComponent` (`self.Homing Target Component`) (`self.ProjectileMovement`)))