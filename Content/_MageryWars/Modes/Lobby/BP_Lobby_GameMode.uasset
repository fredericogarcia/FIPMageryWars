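; Lobby game mode that tracks connected player controllers and their Steam names, and assigns players to lobby spawn-point slots.
; One tick after BeginPlay, it orders BP_Lobby_SpawnPoint actors into slots by their numeric index tags.
; PostLogin and OnLogout update the player lists, then wait through a polling delay macro until slots are ready.
; UpdatePlayerSlot then puts unassigned players in free slots and clears slots of departed players.
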(event `self.ReceiveBeginPlay`
  (`KismetSystemLibrary.DelayUntilNextTick`)
  (`self.SetPlayerSlot`))

(event `self.K2_PostLogin`
  (params (NewPlayer :type "PlayerController Object Reference"))
  (`KismetArrayLibrary.Array_Add` (`self.PlayerControllers`) NewPlayer)
  (bind _returnvalue (`AdvancedSteamFriendsLibrary.GetSteamPersonaName` (`AdvancedSessionsLibrary.GetUniqueNetID` NewPlayer)))
  (`KismetArrayLibrary.Array_Add` (`self.PlayerNames`) _returnvalue)
  (`self.IfPlayerSlotsSet`
    (:`true`
      (`self.UpdatePlayerSlot`))))

(event `self.K2_OnLogout`
  (params (ExitingController :type "Controller Object Reference"))
  (bind _asplayer_controller (cast `PlayerController` ExitingController))
  (`KismetArrayLibrary.Array_RemoveItem` (`self.PlayerControllers`) _asplayer_controller)
  (`KismetArrayLibrary.Array_RemoveItem` (`self.PlayerNames`) (`|GetArrayItem` (`self.PlayerNames`) (`KismetArrayLibrary.Array_Find` (`self.PlayerControllers`) _asplayer_controller)))
  (`self.IfPlayerSlotsSet`
    (:`true`
      (`self.UpdatePlayerSlot`))))

(fn `GetPlayerControllerIndex`
  (params (PlayerController :type "PlayerController Object Reference (by ref)"))
  (returns (Index :type Integer))
  (return (`KismetArrayLibrary.Array_Find` (`self.PlayerControllers`) PlayerController)))

(fn `GetPlayerName`
  (params (`Player Controller` :type "PlayerController Object Reference"))
  (returns (`Player Name` :type "String (by ref)"))
  (return (`|GetArrayItem` (`self.PlayerNames`) (`KismetArrayLibrary.Array_Find` (`self.PlayerControllers`) `Player Controller`))))

(fn `SetPlayerSlot`
  (bind _outactors (`GameplayStatics.GetAllActorsOfClass` "/Game/_MageryWars/Blueprints/BP_Lobby_SpawnPoint.BP_Lobby_SpawnPoint_C"))
  (for _index (range (+ (`KismetArrayLibrary.Array_LastIndex` _outactors) 1))
    (bind _outactors_2 (`GameplayStatics.GetAllActorsOfClassWithTag` "/Game/_MageryWars/Blueprints/BP_Lobby_SpawnPoint.BP_Lobby_SpawnPoint_C" (`KismetStringLibrary.Conv_StringToName` (`KismetStringLibrary.Conv_IntToString` _index))))
    (`KismetArrayLibrary.Array_Add` (`self.PlayerSlots`) (`|GetArrayItem` _outactors_2)))
  (set `self.SetPlayerSlotComplete?` true))

(fn `UpdatePlayerSlot`
  (locals (`PlayerControllerAlreadyAdded?` :type Boolean))
  (for _array_element (`self.PlayerControllers`)
    (set `local.PlayerControllerAlreadyAdded?` false)
    ; Check if already added
    (for _array_element_2 (`self.PlayerSlots`)
      (if (== (`/Game/_MageryWars/Blueprints/BP_Lobby_SpawnPoint.PlayerController` _array_element_2) _array_element)
        (set `local.PlayerControllerAlreadyAdded?` true)
        (break)))
    ; Add
    (if (not (`local.PlayerControllerAlreadyAdded?`))
      (for _array_element_3 (`self.PlayerSlots`)
        (`/Game/_MageryWars/Blueprints/BP_Lobby_SpawnPoint.PlayerController` _array_element_3
          (:`then`)
          (:`else`
            (`/Game/_MageryWars/Blueprints/BP_Lobby_SpawnPoint.Add Player` _array_element_3 _array_element)
            (break))))))
  ; remove
  (for _array_element_4 (`self.PlayerSlots`)
    (if (not (`KismetArrayLibrary.Array_Contains` (`self.PlayerControllers`) (`/Game/_MageryWars/Blueprints/BP_Lobby_SpawnPoint.PlayerController` _array_element_4)))
      (`/Game/_MageryWars/Blueprints/BP_Lobby_SpawnPoint.Remove Player` _array_element_4))))

(fn `UserConstructionScript`)