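; Game state for Magery Wars that tracks arena occupancy and runs duels from countdown to defeat.
; StartDuelTimer plays countdowns, then a delayed announcement starts HUD timers, start-match effects and potion spawners.
; A bound sudden death event applies a GAS effect and HUD warning to all players.
; EndDuel respawns players, resets timers, spawners and portals, with a DoOnce guarding the defeat announcement; DuelStarted's OnRep updates music.
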(event `ResetDuelStart`
  (set `self.DuelStarted` false))

(event `self.ReceiveBeginPlay`
  (add `self.TriggerSuddenDeath` (delegate `SuddenDeath`))
  (`KismetSystemLibrary.Delay` 2.0)
  (`self.ResetDuelStart`))

(event `SuddenDeath`
  (for _array_element (`self.PlayerArray`)
    (bind _asbp_player_character (cast `/Game/_MageryWars/Blueprints/BP_PlayerCharacter` (`PlayerState.PawnPrivate` _array_element)))
    (`AbilitySystemComponent.BP_ApplyGameplayEffectToSelf` :`self` (`AbilitySystemBlueprintLibrary.GetAbilitySystemComponent` _asbp_player_character) :`GameplayEffectClass` "/Game/_MageryWars/Abilities/_Arena/GE_SuddenDeath.GE_SuddenDeath_C")
    (bind _playerhud (`/Game/_MageryWars/Blueprints/BP_PlayerCharacter.PlayerHUD` _asbp_player_character))
    (`/Engine/EditorBlueprintResources/StandardMacros.IsValid` _playerhud
      (:`Is Valid`
        (`/Game/_MageryWars/Widgets/W_SuddenDeath.PlaySuddenDeaht` (`/Game/_MageryWars/Widgets/W_HUD.W_SuddenDeath` _playerhud))
        (`Widget.SetRenderOpacity` (`/Game/_MageryWars/Widgets/W_HUD.SDeath` _playerhud) 1.0)))))

(event `StartDuelAnnouncement`
  (`KismetSystemLibrary.Delay` 12.0)
  (for (_array_element _array_index) (`self.PlayerArray`)
    (bind _asbp_player_controller (cast `/Game/_MageryWars/Blueprints/BP_PlayerController` (`PlayerState.GetPlayerController` _array_element)))
    (bind _w_hud (`/Game/_MageryWars/Blueprints/BP_PlayerController.W_HUD` _asbp_player_controller))
    (`/Engine/EditorBlueprintResources/StandardMacros.IsValid` _w_hud
      (:`Is Valid`
        (`/Game/_MageryWars/Widgets/W_ArenaTimer.StartTimer` (`/Game/_MageryWars/Widgets/W_HUD.W_ArenaTimer` _w_hud))
        (if (== _array_index 0)
          (`self.StartDuel`)
          (bind _asbp_player_character (cast `/Game/_MageryWars/Blueprints/BP_PlayerCharacter` (`PlayerState.PawnPrivate` _array_element)))
          (`/Game/_MageryWars/Blueprints/BP_PlayerCharacter.PlayBackgroundMusic` _asbp_player_character)
          (`/Engine/EditorBlueprintResources/ActorMacros.Switch Has Authority`
            (:`Authority`
              (`/Game/_MageryWars/Blueprints/BP_PlayerController.SERVER_Announcement` _asbp_player_controller "The duel has now begun!")))))))
  (set `self.DuelStarted` true)
  (goto _label :!via `Reset`))

(event `EndDuel`
  (params (PlayerName :type String))
  (`|ExecutionSequence`
    (:`then_0`
      (`/Engine/EditorBlueprintResources/StandardMacros.DoOnce` false :!label _label
        (:`Completed`
          (bind _asbp_player_controller (cast `/Game/_MageryWars/Blueprints/BP_PlayerController` (`PlayerState.GetPlayerController` (`|GetArrayItem` (`self.PlayerArray`)))))
          (`/Game/_MageryWars/Blueprints/BP_PlayerController.SERVER_Announcement` _asbp_player_controller (`|FormatText` "{player} has been defeated!" PlayerName))
          (set `self.DuelStarted` false)
          (set `self.AmountOfPlayersInArena` 0))))
    (:`then_1`
      (for _array_element (`self.PlayerArray`)
        (bind _asbp_player_character (cast `/Game/_MageryWars/Blueprints/BP_PlayerCharacter` (`PlayerState.PawnPrivate` _array_element)))
        (`/Game/_MageryWars/Blueprints/BP_PlayerCharacter.Respawn` _asbp_player_character)
        (bind _asbp_player_controller_2 (cast `/Game/_MageryWars/Blueprints/BP_PlayerController` (`PlayerState.GetPlayerController` _array_element)))
        (bind _w_hud (`/Game/_MageryWars/Blueprints/BP_PlayerController.W_HUD` _asbp_player_controller_2))
        (`/Engine/EditorBlueprintResources/StandardMacros.IsValid` _w_hud
          (:`Is Valid`
            (`/Game/_MageryWars/Widgets/W_ArenaTimer.EndTimer` (`/Game/_MageryWars/Widgets/W_HUD.W_ArenaTimer` _w_hud))
            (`Widget.SetRenderOpacity` (`/Game/_MageryWars/Widgets/W_HUD.SDeath` _w_hud) 0.0)))))
    (:`then_2`
      (bind _outactors (`GameplayStatics.GetAllActorsOfClass` "/Game/_MageryWars/Blueprints/Potions/BP_PotionSpawner.BP_PotionSpawner_C"))
      (for _array_element_2 _outactors
        (`/Game/_MageryWars/Blueprints/Potions/BP_PotionSpawner.StopPotionTimer` _array_element_2)
        (bind _outactors_2 (`GameplayStatics.GetAllActorsOfClass` "/Game/_MageryWars/Blueprints/BP_Portal_Entry_Locator.BP_Portal_Entry_Locator_C"))
        (for _array_element_3 _outactors_2
          (`/Game/_MageryWars/Blueprints/BP_Portal_Entry_Locator.ResetAvailability` _array_element_3))))))

(fn `CheckIfArenaIsFull`
  (params (MaxPlayers :type Integer))
  (returns (Full :type Boolean))
  (if (== MaxPlayers (`self.AmountOfPlayersInArena`))
    (return true)
    (else
      (return false))))

(fn `OnRep_DuelStarted`
  (for _array_element (`self.PlayerArray`)
    (bind _asbp_player_character (cast `/Game/_MageryWars/Blueprints/BP_PlayerCharacter` (`PlayerState.PawnPrivate` _array_element)))
    (`/Game/_MageryWars/Blueprints/BP_PlayerCharacter.PlayBackgroundMusic` _asbp_player_character)))

(fn `StartDuel`
  (for _array_element (`self.PlayerArray`)
    (bind _asbp_player_character (cast `/Game/_MageryWars/Blueprints/BP_PlayerCharacter` (`PlayerState.PawnPrivate` _array_element)))
    (`/Game/_MageryWars/Blueprints/BP_PlayerCharacter.ApplyStartMatchEffect` _asbp_player_character)
    (bind _outactors (`GameplayStatics.GetAllActorsOfClass` "/Game/_MageryWars/Blueprints/Potions/BP_PotionSpawner.BP_PotionSpawner_C"))
    (for _array_element_2 _outactors
      (`/Game/_MageryWars/Blueprints/Potions/BP_PotionSpawner.StartPotionTimer` _array_element_2))))

(fn `StartDuelTimer`
  (for _array_element (`self.PlayerArray`)
    (bind _asbp_player_character (cast `/Game/_MageryWars/Blueprints/BP_PlayerCharacter` (`PlayerState.PawnPrivate` _array_element)))
    (bind _playerhud (`/Game/_MageryWars/Blueprints/BP_PlayerCharacter.PlayerHUD` _asbp_player_character))
    (`/Engine/EditorBlueprintResources/StandardMacros.IsValid` _playerhud
      (:`Is Valid`
        (`/Game/_MageryWars/Widgets/W_ArenaCountDown.PlayCountdown` (`/Game/_MageryWars/Widgets/W_HUD.W_ArenaCountDown` _playerhud))
        (`self.StartDuelAnnouncement`)))))

(fn `UpdateAmountOfPlayersInArena`
  (params (Amount :type Integer))
  (set `self.AmountOfPlayersInArena` (+ (`self.AmountOfPlayersInArena`) Amount)))

(fn `UserConstructionScript`)