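; Core game mode that tracks connected players and their Steam persona names and spawns their characters.
; Login and logout update parallel controller and name arrays, with names gated on the Steam overlay check; logout looks up the name index after removing the controller.
; Each new player gets a character at a PlayerStart, which is then destroyed so it is not reused.
; The character is possessed and receives the Steam name through a multicast.
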(event `self.K2_PostLogin`
  (params (NewPlayer :type "PlayerController Object Reference"))
  (`KismetArrayLibrary.Array_Add` (`self.PlayerControllers`) NewPlayer)
  (if (`AdvancedSteamFriendsLibrary.IsOverlayEnabled`)
    (bind _returnvalue (`AdvancedSteamFriendsLibrary.GetSteamPersonaName` (`AdvancedSessionsLibrary.GetUniqueNetID` NewPlayer)))
    (`KismetArrayLibrary.Array_Add` (`self.PlayerNames`) _returnvalue)))

(event `self.K2_OnLogout`
  (params (ExitingController :type "Controller Object Reference"))
  (bind _playernames (`self.PlayerNames`))
  (bind _asbp_player_controller (cast `/Game/_MageryWars/Blueprints/BP_PlayerController` ExitingController))
  (`KismetArrayLibrary.Array_RemoveItem` (`self.PlayerControllers`) _asbp_player_controller)
  (if (`AdvancedSteamFriendsLibrary.IsOverlayEnabled`)
    (if (`KismetArrayLibrary.Array_IsNotEmpty` _playernames)
      (`KismetArrayLibrary.Array_RemoveItem` (`self.PlayerNames`) (`|GetArrayItem` _playernames (`KismetArrayLibrary.Array_Find` (`self.PlayerControllers`) _asbp_player_controller))))))

(event `self.HandleStartingNewPlayer`
  (params (NewPlayer :type "PlayerController Object Reference"))
  (`/Engine/EditorBlueprintResources/ActorMacros.Switch Has Authority`
    (:`Authority`
      (bind _returnvalue (`GameplayStatics.GetActorOfClass` "/Script/Engine.PlayerStart"))
      (bind _returnvalue_2 (`|SpawnActorFromClass` "/Game/_MageryWars/Blueprints/BP_PlayerCharacter.BP_PlayerCharacter_C" (`self.GetTransform` _returnvalue) "Undefined" "MultiplyWithRoot" NewPlayer null))
      (`self.K2_DestroyActor` _returnvalue)
      (`Controller.Possess` NewPlayer _returnvalue_2)
      (`self.SERVER_SetPlayerName` _returnvalue_2 NewPlayer))))

(event `SERVER_SetPlayerName`
  (params (`Player Character` :type "/Game/_MageryWars/Blueprints/BP_PlayerCharacter Object Reference") (`Player Controller` :type "PlayerController Object Reference"))
  (bind _asbp_player_controller (cast `/Game/_MageryWars/Blueprints/BP_PlayerController` `Player Controller`))
  (bind _returnvalue (`AdvancedSteamFriendsLibrary.GetSteamPersonaName` (`AdvancedSessionsLibrary.GetUniqueNetID` _asbp_player_controller)))
  (`/Game/_MageryWars/Blueprints/BP_PlayerCharacter.MC_SetPlayerName` `Player Character` _returnvalue))

(fn `GetPlayerControllerIndex`
  (params (PlayerController :type "PlayerController Object Reference (by ref)"))
  (returns (Index :type Integer))
  (return (`KismetArrayLibrary.Array_Find` (`self.PlayerControllers`) PlayerController)))

(fn `GetPlayerName`
  (params (`Player Controller` :type "PlayerController Object Reference"))
  (returns (`Player Name` :type "String (by ref)"))
  (return (`|GetArrayItem` (`self.PlayerNames`) (`self.GetPlayerControllerIndex` `Player Controller`))))

(fn `UserConstructionScript`)