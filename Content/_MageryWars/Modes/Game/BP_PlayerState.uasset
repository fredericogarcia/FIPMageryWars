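; BP_PlayerState is the Magery Wars player state that holds each player's Steam name and shows it on their character's name widget.
; One tick after BeginPlay, it reads the Steam persona name from the player controller's unique net ID and passes it to UpdateName, which stores it in SteamName.
; SteamName's RepNotify finds the BP_PlayerCharacter pawn and writes the name into its W_PlayerName widget.
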(event `self.ReceiveBeginPlay`
  (`KismetSystemLibrary.DelayUntilNextTick`)
  (bind _returnvalue (`AdvancedSteamFriendsLibrary.GetSteamPersonaName` (`AdvancedSessionsLibrary.GetUniqueNetID` (`self.GetPlayerController`))))
  (`self.UpdateName` _returnvalue))

(event `UpdateName`
  (params (SteamName :type String))
  (set `self.SteamName` SteamName))

(fn `OnRep_SteamName`
  (bind _asbp_player_character (cast `/Game/_MageryWars/Blueprints/BP_PlayerCharacter` (`self.GetPawn`)))
  (bind _asw_player_name (cast `/Game/_MageryWars/Widgets/W_PlayerName` (`WidgetComponent.GetWidget` (`/Game/_MageryWars/Blueprints/BP_PlayerCharacter.Widget` _asbp_player_character))))
  (`TextBlock.SetText` (`/Game/_MageryWars/Widgets/W_PlayerName.PlayerName` _asw_player_name) (`KismetTextLibrary.Conv_StringToText` (`self.SteamName`))))

(fn `UserConstructionScript`)